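; HUD Blueprint for the Lab 4 guide game that shows score, time and player level, plus a game-over prompt.
; On BeginPlay it casts and caches the BP_Guide_GameMode_Lab4 game mode.
; Each DrawHUD pass reads that game mode's values and draws them as colored canvas text along the top, adding "GAME OVER" and "PRESS ENTER" when its GameOver flag is set.
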(event `self.ReceiveBeginPlay`
  (bind _asbp_guide_game_mode_lab_4 (cast `/Game/1906832-Lab4/BP_Guide_GameMode_Lab4` (`GameplayStatics.GetGameMode`)))
  (set `self.My_Guide_GameMode` _asbp_guide_game_mode_lab_4))

(event `self.ReceiveDrawHUD`
  (params (SizeX :type Integer) (SizeY :type Integer))
  (`self.DrawText` (`KismetStringLibrary.BuildString_Int` "Score:" "" (`/Game/1906832-Lab4/BP_Guide_GameMode_Lab4.Score` (`self.My_Guide_GameMode`))) (struct :`R` 1.0 :`G` 0.834771 :`A` 1.0) 10.0 10.0 null 3.0)
  (`self.DrawText` (`KismetStringLibrary.BuildString_Int` "Time:" "" (`/Game/1906832-Lab4/BP_Guide_GameMode_Lab4.Time` (`self.My_Guide_GameMode`))) (struct :`R` 1.0 :`G` 0.052026 :`B` 0.061973 :`A` 1.0) 300.0 10.0 null 3.0)
  (`self.DrawText` (`KismetStringLibrary.BuildString_Int` "Player Level:" "" (`/Game/1906832-Lab4/BP_Guide_GameMode_Lab4.Level` (`self.My_Guide_GameMode`))) (struct :`R` 0.066928 :`B` 1.0 :`A` 1.0) 550.0 10.0 null 3.0)
  (if (`/Game/1906832-Lab4/BP_Guide_GameMode_Lab4.GameOver` (`self.My_Guide_GameMode`))
    (`self.DrawText` "GAME OVER" (struct :`R` 1.0 :`B` 0.044042 :`A` 1.0) 400.0 200.0 null 3.0)
    (`self.DrawText` "PRESS ENTER" (struct :`R` 1.0 :`B` 0.022732 :`A` 1.0) 400.0 400.0 null 3.0)))

(fn `UserConstructionScript`)