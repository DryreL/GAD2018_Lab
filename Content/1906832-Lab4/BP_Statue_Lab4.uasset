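; BP_Statue_Lab4 is a collectible statue that jumps around the level until the player touches it.
; InitStatue teleports it to a random X/Y at fixed height, then re-arms itself on a timer whose delay in seconds equals the game mode's Level.
; When the player overlaps it before game over, it notifies the game mode, destroys itself and spawns a replacement, which randomizes its position on BeginPlay.
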(event `self.ReceiveBeginPlay`
  (bind _asbp_guide_game_mode_lab_4 (cast `/Game/1906832-Lab4/BP_Guide_GameMode_Lab4` (`GameplayStatics.GetGameMode`)))
  (set `self.As BP Guide Game Mode` _asbp_guide_game_mode_lab_4)
  (`self.InitStatue`))

(event `self.ReceiveActorBeginOverlap`
  (params (OtherActor :type "Actor Object Reference"))
  (if (and (== OtherActor (`GameplayStatics.GetPlayerCharacter` 0)) (not (`/Game/1906832-Lab4/BP_Guide_GameMode_Lab4.GameOver` (`self.As BP Guide Game Mode`))))
    (`/Game/1906832-Lab4/BP_Guide_GameMode_Lab4.Statue Collected` (`self.As BP Guide Game Mode`))
    (`self.K2_DestroyActor`)
    (`|SpawnActorFromClass` "BP_Statue_Lab4_C" (`self.GetTransform`) "Undefined" "OverrideRootScale" null null)))

(fn `InitStatue`
  (`self.K2_TeleportTo` (`KismetMathLibrary.MakeVector` (`KismetMathLibrary.RandomFloatInRange` -1800.0 1800.0) (`KismetMathLibrary.RandomFloatInRange` -1400.0 1400.0) 130.0))
  (`KismetSystemLibrary.K2_SetTimer` null "InitStatue" (`KismetMathLibrary.Conv_IntToDouble` (`/Game/1906832-Lab4/BP_Guide_GameMode_Lab4.Level` (`self.As BP Guide Game Mode`)))))

(fn `UserConstructionScript`)