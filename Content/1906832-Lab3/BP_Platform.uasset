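; BP_Platform is a self-chaining walled track segment with a spinning collectible coin, forming an endlessly generated path.
; The construction script sizes the floor and walls from PlatformLength and places the coin randomly along the segment.
; A DoOnce, reset shortly after BeginPlay, lets a SpawnArea overlap spawn the next platform at the far end with random length, pitch and stepped yaw.
; Tick spins the coin until the character collects it, which disables ticking.
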(event `self.ReceiveBeginPlay`
  (bind (_returnvalue_roll _returnvalue_pitch _returnvalue_yaw) (`KismetMathLibrary.BreakRotator` (`self.K2_GetActorRotation`)))
  (`KismetSystemLibrary.Delay` 0.2)
  (goto _label :!via `Reset`))

(event `self.ReceiveActorBeginOverlap`
  (params (OtherActor :type "Actor Object Reference")))

(event `self.SpawnArea.OnComponentBeginOverlap`
  (params (OverlappedComponent :type "PrimitiveComponent Object Reference") (OtherActor :type "Actor Object Reference") (OtherComp :type "PrimitiveComponent Object Reference") (OtherBodyIndex :type Integer) (bFromSweep :type Boolean) (SweepResult :type "HitResult Structure (by ref)"))
  (bind (_returnvalue_roll _returnvalue_pitch _returnvalue_yaw) (`KismetMathLibrary.BreakRotator` (`self.K2_GetActorRotation`)))
  (`/Engine/EditorBlueprintResources/StandardMacros.DoOnce` true :!label _label
    (:`Completed`
      (`|SpawnActorFromClass` "BP_Platform_C" (`KismetMathLibrary.MakeTransform` (+ (`self.K2_GetActorLocation`) (* (`self.GetActorForwardVector`) (* 100.0 (`self.PlatformLength`)))) (`KismetMathLibrary.MakeRotator` 0.0 (`KismetMathLibrary.Conv_IntToDouble` (`KismetMathLibrary.RandomIntegerInRange` -25 25)) (+ _returnvalue_yaw (* (`KismetMathLibrary.Conv_IntToDouble` (`KismetMathLibrary.RandomIntegerInRange` -3 3)) 15.0)))) "Undefined" "OverrideRootScale" null (`KismetMathLibrary.Conv_IntToDouble` (`KismetMathLibrary.RandomIntegerInRange` 5 15)) null))))

(event `self.Coin.OnComponentBeginOverlap`
  (params (OverlappedComponent :type "PrimitiveComponent Object Reference") (OtherActor :type "Actor Object Reference") (OtherComp :type "PrimitiveComponent Object Reference") (OtherBodyIndex :type Integer) (bFromSweep :type Boolean) (SweepResult :type "HitResult Structure (by ref)"))
  ;[0.3926 1 0.4024] Collect and Rotate Coin
  (cast `/Game/1906832-Lab3/ThirdPersonCharacter_Lab3` OtherActor)
  (`ActorComponent.K2_DestroyComponent` (`self.Coin`))
  (`self.SetActorTickEnabled` false))

(event `self.ReceiveTick`
  (params (DeltaSeconds :type "Float (single-precision)"))
  ;[0.3926 1 0.4024] Collect and Rotate Coin
  (`SceneComponent.K2_AddRelativeRotation` (`self.Coin`) (`KismetMathLibrary.MakeRotator` 0.0 0.0 (* DeltaSeconds 360.0)) false false))

(fn `UserConstructionScript`
  (bind _platformlength (`self.PlatformLength`))
  (`SceneComponent.SetRelativeScale3D` (`self.Floor`) (`KismetMathLibrary.MakeVector` _platformlength 2.0 0.1))
  (`SceneComponent.SetRelativeScale3D` (`self.RightWall`) (`KismetMathLibrary.MakeVector` _platformlength 0.1 2.0))
  (`SceneComponent.SetRelativeScale3D` (`self.LeftWall`) (`KismetMathLibrary.MakeVector` _platformlength 0.1 2.0))
  (`SceneComponent.K2_AddRelativeLocation` (`self.Floor`) (`KismetMathLibrary.MakeVector` (* (`self.PlatformLength`) 50.0)) false false)
  (`SceneComponent.K2_AddRelativeLocation` (`self.SpawnArea`) (`KismetMathLibrary.MakeVector` (* (`self.PlatformLength`) 50.0)) false false)
  (`SceneComponent.K2_AddRelativeLocation` (`self.RightWall`) (`KismetMathLibrary.MakeVector` (* (`self.PlatformLength`) 50.0)) false false)
  (`SceneComponent.K2_AddRelativeLocation` (`self.LeftWall`) (`KismetMathLibrary.MakeVector` (* (`self.PlatformLength`) 50.0)) false false)
  (`SceneComponent.K2_AddRelativeLocation` (`self.Coin`) (`KismetMathLibrary.MakeVector` (`KismetMathLibrary.RandomFloatInRange` 30.0 (* (`self.PlatformLength`) 100.0)) (`KismetMathLibrary.RandomFloatInRange` -50.0 50.0)) false false))