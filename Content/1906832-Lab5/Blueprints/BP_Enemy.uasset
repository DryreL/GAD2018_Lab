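; BP_Enemy is a side-scroller enemy that patrols along the Y axis, damages the player and can be stomped.
; Tick moves it and uses two line traces, for ledges at its feet and walls ahead, to update walk direction.
; HitBox overlap damages the player unless Dead is set.
; HurtBox overlap by a falling player calls AddScore with that player's Score, plays a death sound and destroys the enemy.
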(event `self.HitBox.OnComponentBeginOverlap`
  (params (OverlappedComponent :type "PrimitiveComponent Object Reference") (OtherActor :type "Actor Object Reference") (OtherComp :type "PrimitiveComponent Object Reference") (OtherBodyIndex :type Integer) (bFromSweep :type Boolean) (SweepResult :type "HitResult Structure (by ref)"))
  ;[0.09369 0.9901 1] Lab5 - Overlaps
  (if (not (`self.Dead`))
    (bind _asside_scroller_character_lab_5 (cast `/Game/1906832-Lab5/Blueprints/SideScrollerCharacter_Lab5` OtherActor))
    (`GameplayStatics.ApplyDamage` _asside_scroller_character_lab_5 1.0)))

(event `self.HurtBox.OnComponentBeginOverlap`
  (params (OverlappedComponent :type "PrimitiveComponent Object Reference") (OtherActor :type "Actor Object Reference") (OtherComp :type "PrimitiveComponent Object Reference") (OtherBodyIndex :type Integer) (bFromSweep :type Boolean) (SweepResult :type "HitResult Structure (by ref)"))
  ;[0.09369 0.9901 1] Lab5 - Overlaps
  (bind _asside_scroller_character_lab_5 (cast `/Game/1906832-Lab5/Blueprints/SideScrollerCharacter_Lab5` OtherActor))
  (bind (_returnvalue_x _returnvalue_y _returnvalue_z) (`KismetMathLibrary.BreakVector` (`self.GetVelocity` _asside_scroller_character_lab_5)))
  (if (< _returnvalue_z 0.0)
    (`/Game/1906832-Lab5/Blueprints/SideScrollerCharacter_Lab5.AddScore` _asside_scroller_character_lab_5 (`/Game/1906832-Lab5/Blueprints/SideScrollerCharacter_Lab5.Score` _asside_scroller_character_lab_5))
    (`self.PlayAnimMontage` null)
    (`GameplayStatics.PlaySoundAtLocation` "/Game/1906832-Lab5/SFX/MaleDeathSound1_wav.MaleDeathSound1_wav" (`SceneComponent.K2_GetComponentLocation` (`self.SkeletalMesh`)) (struct) 1.0 1.0 0.0 null null null)
    (`self.K2_DestroyActor`)))

(event `self.ReceiveTick`
  (params (DeltaSeconds :type "Float (single-precision)"))
  (bind _returnvalue (`self.K2_GetActorLocation`))
  (bind _returnvalue_2 (+ (`SceneComponent.K2_GetComponentLocation` (`self.Mesh`)) (`KismetMathLibrary.MakeVector` 0.0 (* (`self.WalkDirection`) 10.0))))
  ;[0.07485 0.8803 1] Lab5 - Enemy Walks
  (`self.AddMovementInput` (`KismetMathLibrary.MakeVector` 0.0 (`self.WalkDirection`)) (* DeltaSeconds (`self.WalkSpeed`)))
  ;[0 0.9274 1] Lab5 - FeetCheck
  (bind (_outhit _returnvalue_3) (`KismetSystemLibrary.LineTraceSingle` _returnvalue_2 (+ _returnvalue_2 (0.0 0.0 -100.0)) "TraceTypeQuery1"))
  (if _returnvalue_3
    ;[0.03125 1 1] Lab5 - WallCheck
    (bind (_outhit_2 _returnvalue_4) (`KismetSystemLibrary.LineTraceSingle` _returnvalue (+ _returnvalue (`KismetMathLibrary.MakeVector` 0.0 (* (`self.WalkDirection`) (`self.WalkSpeed`) 2.0))) "TraceTypeQuery1"))
    (if _returnvalue_4
      (`/Engine/EditorBlueprintResources/StandardMacros.NegateFloat` (`self.WalkDirection`)))
    (else
      (`/Engine/EditorBlueprintResources/StandardMacros.NegateFloat` (`self.WalkDirection`)))))

(fn `UserConstructionScript`)