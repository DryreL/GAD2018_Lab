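; BP_HUD_Lab5 is the on-screen HUD for the Lab 5 side-scroller, showing the player's hit points and score.
; Each DrawHUD call casts the player character to SideScrollerCharacter_Lab5 and reads its HitPoints and Score directly.
; It draws a row of evenly spaced heart textures, one per hit point, and a gold "Score:" label with the current value, using immediate-mode canvas drawing rather than widgets.
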(event `self.ReceiveDrawHUD`
  (params (SizeX :type Integer) (SizeY :type Integer))
  ;[0.1962 1 0.9502] Lab5
  (bind _asside_scroller_character_lab_5 (cast `/Game/1906832-Lab5/Blueprints/SideScrollerCharacter_Lab5` (`GameplayStatics.GetPlayerCharacter` 0)))
  (for _index (range 1 (+ (`/Game/1906832-Lab5/Blueprints/SideScrollerCharacter_Lab5.HitPoints` _asside_scroller_character_lab_5) 1))
    (`self.DrawTextureSimple` "/Game/1906832-Lab5/Sprites/Heart.Heart" (`KismetMathLibrary.Conv_IntToDouble` (+ (* _index 45) 10)) 15.0 0.01))
  (`self.DrawText` (`KismetStringLibrary.BuildString_Int` "Score: " "" (`/Game/1906832-Lab5/Blueprints/SideScrollerCharacter_Lab5.Score` _asside_scroller_character_lab_5)) (struct :`R` 1.0 :`G` 0.729969 :`A` 1.0) 225.0 10.0 "/Game/1906832-Lab5/Fonts/Exo2-Bold_Font.Exo2-Bold_Font" 3.0))

(fn `UserConstructionScript`)