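; BP_MovingPlatform_Lab5 is a platform actor whose cube mesh moves along a configurable offset.
; On BeginPlay, the MovePlatform timeline plays at PlayRate, and its Amount track scales the Movement variable to set the cube's relative location without sweeping.
; The construction script sets the cube's Y scale from Length, with X and Z scale set to zero.
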(event `self.ReceiveBeginPlay`
  (`TimelineComponent.SetPlayRate` (`self.MovePlatform`) (`self.PlayRate`))
  (bind (_direction _amount) (`Timeline|MovePlatform`)
    (:`Update`
      (`SceneComponent.K2_SetRelativeLocation` (`self.1M_Cube`) (* (`self.Movement`) _amount) false false))))

(fn `UserConstructionScript`
  (`SceneComponent.SetRelativeScale3D` (`self.1M_Cube`) (`KismetMathLibrary.MakeVector` 0.0 (`self.Length`))))