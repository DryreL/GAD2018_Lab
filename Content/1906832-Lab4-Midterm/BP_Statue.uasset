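; BP_Statue is a collectible that jumps to random spots within a fixed area and, when the player touches it before game over, notifies BP_Guide_GameMode.
; InitStatue runs at BeginPlay, teleports the statue, re-arms itself by timer using the game mode's Level as delay, and shows Level as colored text.
; On collection it destroys itself and spawns a replacement, whose BeginPlay picks a new position.
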(event `self.ReceiveBeginPlay`
  (bind _asbp_guide_game_mode (cast `/Game/1906832-Lab4-Midterm/BP_Guide_GameMode` (`GameplayStatics.GetGameMode`)))
  (set `self.As BP Guide Game Mode` _asbp_guide_game_mode)
  (`self.InitStatue`))

(event `self.ReceiveActorBeginOverlap`
  (params (OtherActor :type "Actor Object Reference"))
  (if (and (== OtherActor (`GameplayStatics.GetPlayerCharacter` 0)) (not (`/Game/1906832-Lab4-Midterm/BP_Guide_GameMode.GameOver` (`self.As BP Guide Game Mode`))))
    (`/Game/1906832-Lab4-Midterm/BP_Guide_GameMode.Statue Collected` (`self.As BP Guide Game Mode`))
    (`self.K2_DestroyActor`)
    (`|SpawnActorFromClass` "BP_Statue_C" (`self.GetTransform`) "Undefined" "OverrideRootScale" null null)))

(fn `InitStatue`
  (locals (NewLocalVar_0 :type Integer :default 0))
  (bind _returnvalue (`KismetMathLibrary.Conv_IntToDouble` (`/Game/1906832-Lab4-Midterm/BP_Guide_GameMode.Level` (`self.As BP Guide Game Mode`))))
  (`self.K2_TeleportTo` (`KismetMathLibrary.MakeVector` (`KismetMathLibrary.RandomFloatInRange` -1800.0 1800.0) (`KismetMathLibrary.RandomFloatInRange` -1400.0 1400.0) 130.0))
  (`KismetSystemLibrary.K2_SetTimer` "BP_Statue" "InitStatue" _returnvalue)
  (if (`self.IsActorBeingDestroyed`)
    (`KismetSystemLibrary.PrintString` "BP_Statue Destroyed")
    (else
      (`TextRenderComponent.K2_SetText` (`self.BP_Statue_Text`) (`KismetTextLibrary.Conv_DoubleToText` _returnvalue "HalfToEven"))
      (if (< _returnvalue 1.0)
        (`TextRenderComponent.SetTextRenderColor` (`self.BP_Statue_Text`) (make `Color` 0 0 255))
        (else
          (`TextRenderComponent.SetTextRenderColor` (`self.BP_Statue_Text`) (make `Color` 0 255)))))))

(fn `UserConstructionScript`)