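; BP_Trap is a trap actor that briefly freezes the player when something overlaps it.
; Each tick it reads TrapActive on the player's ThirdPersonCharacter to show or hide the trap and toggle its box collision.
; On overlap it enlarges itself, spawns an explosion, disables player input for a short delay and prints trapped and escaped messages.
; The overlap does not check which actor entered, always targeting player 0.
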(event `self.ReceiveTick`
  (params (DeltaSeconds :type "Float (single-precision)"))
  ;[0.2814 1 0.1527] Midterm Blueprint - Trap
  (bind _asthird_person_character (cast `/Game/1906832-Lab4-Midterm/ThirdPersonCharacter` (`GameplayStatics.GetPlayerPawn` 0)))
  (bind _output_get (set `self.As Third Person Character` _asthird_person_character))
  (if (`/Game/1906832-Lab4-Midterm/ThirdPersonCharacter.TrapActive` _output_get)
    (`SceneComponent.SetVisibility` (`self.Trap`) true false)
    (`PrimitiveComponent.SetCollisionEnabled` (`self.Box Collision`) "QueryAndPhysics")
    (else
      (`SceneComponent.SetVisibility` (`self.Trap`) false false)
      (`PrimitiveComponent.SetCollisionEnabled` (`self.Box Collision`) "NoCollision"))))

(event `self.ReceiveActorBeginOverlap`
  (params (OtherActor :type "Actor Object Reference"))
  (bind _returnvalue (`GameplayStatics.GetPlayerPawn` 0))
  ;[0.2814 1 0.1527] Midterm Blueprint - Trap
  (`self.SetActorScale3D` (+ (`SceneComponent.K2_GetComponentScale` (`self.Trap`)) (0.5 0.5 1.0)))
  (`GameplayStatics.SpawnEmitterAtLocation` "/Game/StarterContent/Particles/P_Explosion.P_Explosion" (`SceneComponent.K2_GetComponentLocation` (`self.Trap`)))
  (`self.DisableInput` _returnvalue null)
  (`KismetSystemLibrary.PrintString` "UNLUCKY! You got trapped. (you are frozen for 2 seconds)" true true (struct :`R` 1.0 :`A` 1.0))
  (`KismetSystemLibrary.Delay` 2.0)
  (`self.EnableInput` _returnvalue null)
  (`KismetSystemLibrary.PrintString` "You escaped from trap! Come on, continue!" true true (struct :`G` 1.0 :`B` 0.33547 :`A` 1.0)))

(fn `UserConstructionScript`)