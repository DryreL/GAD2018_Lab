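; BP_BasicItem is a data-driven item actor that can be taken, left and thrown.
; On construction and BeginPlay, it reads its DT_ItemsRegistry row to set mesh, material and collision, deriving scale from mesh bounds when a metric size is given.
; TakeLeave toggles the collision component's Pawn response.
; Throw launches the mesh with a physics velocity impulse, and Hit stops simulation after a short delay.
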(event `self.ReceiveHit`
  (params (MyComp :type "PrimitiveComponent Object Reference") (Other :type "Actor Object Reference") (OtherComp :type "PrimitiveComponent Object Reference") (bSelfMoved :type Boolean) (HitLocation :type "Vector Structure") (HitNormal :type "Vector Structure") (NormalImpulse :type "Vector Structure") (Hit :type "HitResult Structure (by ref)"))
  (`KismetSystemLibrary.Delay` 2.0)
  (`PrimitiveComponent.SetSimulatePhysics` (`self.Mesh`) false))

(event `self.ReceiveBeginPlay`
  (`self.InitItemProperties`))

(fn `InitItemProperties`
  (bind (_itemid_datatable _itemid_rowname) (break `DataTableRowHandle` (`self.itemid`)))
  (bind _collision (`self.Collision`))
  (bind _mesh (`self.Mesh`))
  (bind (_id _description _mesh_2 _material _icon _heal _weight _throwable _equipable _sizeinmeters _scale _blocktype _acquiredistance _collisionscale _attachoffset _usemeshcollision) (break `/Game/1906832-Lab7/Blueprints/S_InventoryItem` (`self.data`)))
  (bind _returnvalue (`|GetDataTableRow` "/Game/1906832-Lab7/Blueprints/DT_ItemsRegistry.DT_ItemsRegistry" _itemid_rowname)
    (:`then`
      (set `self.data` _returnvalue)
      (`SceneComponent.SetWorldScale3D` _mesh (select `bool` (== (`KismetMathLibrary.VSize` _sizeinmeters) 0.0) :`false` (/ (* _sizeinmeters 100.0) (* (`.BoxExtent` (`KismetMathLibrary.BreakBoxSphereBounds` (`StaticMesh.GetBounds` _mesh_2))) 2.0)) :`true` _scale))
      (`StaticMeshComponent.SetStaticMesh` _mesh _mesh_2)
      (`PrimitiveComponent.SetMaterial` _mesh 0 _material)
      (`PrimitiveComponent.SetCollisionResponseToChannel` _collision "ECC_Visibility" (select `bool` _usemeshcollision :`false` "ECR_Block" :`true` "ECR_Ignore" :!type "ECollisionResponse Enum"))
      (`PrimitiveComponent.SetCollisionResponseToChannel` (`self.Mesh`) "ECC_Visibility" (select `bool` _usemeshcollision :`false` "ECR_Ignore" :`true` "ECR_Block" :!type "ECollisionResponse Enum"))
      (`PrimitiveComponent.SetCollisionResponseToChannel` _collision "ECC_Pawn" _blocktype)
      (`SceneComponent.SetRelativeScale3D` (`self.Collision`) (`KismetMathLibrary.Conv_DoubleToVector` _collisionscale)))))

(fn `TakeLeave`
  (params (`taken?` :type Boolean))
  (bind _collision (`self.Collision`))
  (if `taken?`
    (`PrimitiveComponent.SetCollisionResponseToChannel` _collision "ECC_Pawn" "ECR_Ignore")
    (else
      (`PrimitiveComponent.SetCollisionResponseToChannel` _collision "ECC_Pawn" (`.blocktype_25_043880974585BB25B1DAE3BEEEA3E685` (break `/Game/1906832-Lab7/Blueprints/S_InventoryItem` (`self.data`)))))))

(fn `Throw`
  (params (Impulse :type "Vector Structure"))
  (bind _mesh (`self.Mesh`))
  (`PrimitiveComponent.SetCollisionResponseToChannel` _mesh "ECC_WorldStatic" "ECR_Block")
  (`PrimitiveComponent.SetCollisionEnabled` _mesh "QueryAndPhysics")
  (`PrimitiveComponent.SetSimulatePhysics` _mesh true)
  (`PrimitiveComponent.AddImpulse` _mesh Impulse "None" true))

(fn `UserConstructionScript`
  (`self.InitItemProperties`))