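; BP_Chest is a chest actor that tracks which BP_BasicItem actors are placed in it through the character's inventory.
; On BeginPlay it caches the first ChestGameCharacter in the level.
; Overlap begin adds the item to that character's inventory, and overlap end removes it.
; Disconnected leftover test code for game mode flags, debug prints and a HUD widget never runs.
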(event `self.ReceiveBeginPlay`
  (`|ExecutionSequence`
    (:`then_0`
      (bind _outactors (`GameplayStatics.GetAllActorsOfClass` "/Game/1906832-Lab7/Blueprints/ChestGameCharacter.ChestGameCharacter_C"))
      (set `self.Char Ref` (`|GetArrayItem` _outactors)))))

(event `self.ReceiveActorBeginOverlap`
  (params (OtherActor :type "Actor Object Reference"))
  (bind _asbp_basic_item (cast `/Game/1906832-Lab7/Blueprints/BP_BasicItem` OtherActor))
  (`/Game/1906832-Lab7/Blueprints/ChestGameCharacter.AddtoInventory` (`self.Char Ref`) _asbp_basic_item))

(event `self.ReceiveActorEndOverlap`
  (params (OtherActor :type "Actor Object Reference"))
  (bind _asbp_basic_item (cast `/Game/1906832-Lab7/Blueprints/BP_BasicItem` OtherActor))
  (`/Game/1906832-Lab7/Blueprints/ChestGameCharacter.RemovefromInventory` (`self.Char Ref`) _asbp_basic_item))

(fn `UserConstructionScript`)